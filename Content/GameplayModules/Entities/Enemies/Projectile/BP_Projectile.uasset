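; BP_Projectile is an enemy projectile that flies straight along its spawn forward vector and damages the player through PlayerCombat on overlap.
; Tick performs a swept move by Speed times a timeline-driven multiplier, unscaled by delta time, and plays a one-shot Wwise flyby near the player.
; It destroys itself with break sounds on any overlap or box hit, or once Lifetime elapses after the timeline finishes.
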(event `self.ReceiveBeginPlay`
  ;[1 1 1] Projectile Fire + Beam Sound
  (`AkGameplayStatics.PostEvent` "/Game/WwiseAudio/Events/Default_Work_Unit/Ai_Behavior/Play_EnemyProjectileFire.Play_EnemyProjectileFire" self)
  (`AkGameplayStatics.PostEvent` "/Game/WwiseAudio/Events/Default_Work_Unit/Ai_Behavior/Play_EnemyProjectileBeam.Play_EnemyProjectileBeam" self)
  (set `self.Direction` (`self.GetActorForwardVector`))
  (bind (_direction _newtrack_0) (`Timeline|SpeedTimeline`)
    (:`Update`
      (set `self.SpeedMultiplier` _newtrack_0))
    (:`Finished`
      (`KismetSystemLibrary.Delay` (`self.Lifetime`))
      (if (`KismetSystemLibrary.IsValid` self)
        (`AkGameplayStatics.PostEvent` "/Game/WwiseAudio/Events/Default_Work_Unit/Ai_Behavior/Play_EnemyProjectileBreak.Play_EnemyProjectileBreak" self)
        (`self.K2_DestroyActor`)))))

(event `self.ReceiveTick`
  (params (DeltaSeconds :type "Float (single-precision)"))
  (`self.K2_SetActorLocation` (+ (`self.K2_GetActorLocation`) (* (`self.Direction`) (* (`self.Speed`) (`self.SpeedMultiplier`)))) true)
  ;[1 1 1] Projectile Flyby Sound
  (if (< (`self.GetDistanceTo` (`GameplayStatics.GetPlayerPawn` 0)) 450.0)
    (`/Engine/EditorBlueprintResources/StandardMacros.DoOnce` false
      (:`Completed`
        (`AkGameplayStatics.PostEvent` "/Game/WwiseAudio/Events/Default_Work_Unit/Ai_Behavior/Play_EnemyProjectileFlyby.Play_EnemyProjectileFlyby" self)))))

(event `self.ReceiveActorBeginOverlap`
  (params (OtherActor :type "Actor Object Reference"))
  (bind _returnvalue (`GameplayStatics.GetPlayerCharacter` 0))
  (if (== OtherActor _returnvalue)
    (bind _asred_blood_sea_character (cast `RedBloodSeaCharacter` _returnvalue))
    (`PlayerCombat.DamagePlayer` (`self.GetComponentByClass` _asred_blood_sea_character "/Script/RedBloodSea.PlayerCombat") (`self.Damage Amount`) self)
    ;[1 1 1] Play projectile break sound on player
    (`AkGameplayStatics.PostEvent` "/Game/WwiseAudio/Events/Default_Work_Unit/Ai_Behavior/Play_EnemyProjectileBreak.Play_EnemyProjectileBreak" self)
    (`AkGameplayStatics.PostEvent` "/Game/WwiseAudio/Events/Default_Work_Unit/Ai_Behavior/Play_EnemyProjectileHitPlayer.Play_EnemyProjectileHitPlayer")
    (`self.K2_DestroyActor`)
    (else
      ;[1 1 1] Play projectile break sound on enviro
      (`AkGameplayStatics.PostEvent` "/Game/WwiseAudio/Events/Default_Work_Unit/Ai_Behavior/Play_EnemyProjectileBreak.Play_EnemyProjectileBreak" self :!label _label)
      (`AkGameplayStatics.PostEvent` "/Game/WwiseAudio/Events/Default_Work_Unit/Ai_Behavior/Play_EnemyProjectileHitEnviro.Play_EnemyProjectileHitEnviro" self)
      (`self.K2_DestroyActor`))))

(event `self.Box.OnComponentHit`
  (params (HitComponent :type "PrimitiveComponent Object Reference") (OtherActor :type "Actor Object Reference") (OtherComp :type "PrimitiveComponent Object Reference") (NormalImpulse :type "Vector Structure") (Hit :type "HitResult Structure (by ref)"))
  (goto _label))

(fn `UserConstructionScript`)