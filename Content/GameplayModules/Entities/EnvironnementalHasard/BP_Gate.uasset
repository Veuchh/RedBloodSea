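; BP_Gate is an environmental gate actor that opens and closes through ToggleGate, where a true state means closed.
; On BeginPlay it caches the skeletal mesh's AB_Gate anim instance and the Box's starting relative position.
; Toggling waits a tick, updates the animation and actor collision, and posts Wwise basalt gate sounds, adding an idle sound above the gate when opening.
; A timeline plays or reverses to offset the Box from its base position.
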(event `self.ReceiveBeginPlay`
  (bind _asab_gate (cast `/Game/GameplayModules/Entities/EnvironnementalHasard/AB_Gate` (`SkeletalMeshComponent.GetAnimInstance` (`self.SM_Gate`))))
  (set `self.As AB Gate` _asab_gate)
  (set `self.BaseRelPos` (`SceneComponent.RelativeLocation` (`self.Box`))))

(event `ToggleGate`
  (params (State :type Boolean))
  (bind _returnvalue (`SceneComponent.K2_GetComponentLocation` (`self.SM_Gate`)))
  (`KismetSystemLibrary.DelayUntilNextTick`)
  (`/Game/GameplayModules/Entities/EnvironnementalHasard/AB_Gate.Toggle` (`self.As AB Gate`) State)
  (`self.SetActorEnableCollision` State)
  (if State
    (`KismetSystemLibrary.PrintString` "Gate Close")
    (`AkGameplayStatics.PostEventAtLocation` "/Game/WwiseAudio/Events/Default_Work_Unit/Play_BasaltGate_Close.Play_BasaltGate_Close" _returnvalue)
    (bind (_direction _gateoffset) (`Timeline|Timeline` :!via `Reverse` :!label _label)
      (:`Update`
        (`SceneComponent.K2_SetRelativeLocation` (`self.Box`) (+ _gateoffset (`self.BaseRelPos`)) false false)))
    (else
      (`KismetSystemLibrary.PrintString` "Gate Open")
      (`AkGameplayStatics.PostEventAtLocation` "/Game/WwiseAudio/Events/Default_Work_Unit/Play_BasaltGate_Open.Play_BasaltGate_Open" _returnvalue)
      (`AkGameplayStatics.PostEventAtLocation` "/Game/WwiseAudio/Events/Default_Work_Unit/Play_BasaltGate_Idle.Play_BasaltGate_Idle" (`KismetMathLibrary.MakeVector` (.x _returnvalue) (.y _returnvalue) (+ (.z _returnvalue) 200.0)))
      (goto _label))))

(fn `UserConstructionScript`)