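; BP_SettingsApplier is a utility Blueprint that applies saved RedBloodSea user settings on BeginPlay.
; It sets fullscreen or windowed mode, applies resolution settings, and turns VSync on regardless of any saved value.
; It also pushes the custom blood color and high-contrast options into the MPC_FSEffect material parameter collection as scalar parameters, with toggles written as 1 or 0.
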(event `self.ReceiveBeginPlay`
  (bind _returnvalue (`RedBloodSeaUserSettings.GetRedBloodSeaUserSettings`))
  (if (`RedBloodSeaUserSettings.Fullscreen` _returnvalue)
    (`GameUserSettings.SetFullscreenMode` _returnvalue "Fullscreen")
    (else
      (`GameUserSettings.SetFullscreenMode` _returnvalue "Windowed")))
  (`GameUserSettings.ApplyResolutionSettings` _returnvalue false)
  (if (`RedBloodSeaUserSettings.UseCustomBloodColor` _returnvalue)
    (`KismetMaterialLibrary.SetScalarParameterValue` "/Game/Art/VFX/Mats/PostProcess/MPC_FSEffect.MPC_FSEffect" "UseCustomBloodColor" 1.0)
    (else
      (`KismetMaterialLibrary.SetScalarParameterValue` "/Game/Art/VFX/Mats/PostProcess/MPC_FSEffect.MPC_FSEffect" "UseCustomBloodColor")))
  (`KismetMaterialLibrary.SetScalarParameterValue` "/Game/Art/VFX/Mats/PostProcess/MPC_FSEffect.MPC_FSEffect" "CustomBloodColor_R" (`RedBloodSeaUserSettings.BloodColorRed` _returnvalue))
  (`KismetMaterialLibrary.SetScalarParameterValue` "/Game/Art/VFX/Mats/PostProcess/MPC_FSEffect.MPC_FSEffect" "CustomBloodColor_G" (`RedBloodSeaUserSettings.BloodColorGreen` _returnvalue))
  (`KismetMaterialLibrary.SetScalarParameterValue` "/Game/Art/VFX/Mats/PostProcess/MPC_FSEffect.MPC_FSEffect" "CustomBloodColor_B" (`RedBloodSeaUserSettings.BloodColorBlue` _returnvalue))
  (if (`RedBloodSeaUserSettings.HighContrastMode` _returnvalue)
    (`KismetMaterialLibrary.SetScalarParameterValue` "/Game/Art/VFX/Mats/PostProcess/MPC_FSEffect.MPC_FSEffect" "ToggleHighContrast" 1.0)
    (else
      (`KismetMaterialLibrary.SetScalarParameterValue` "/Game/Art/VFX/Mats/PostProcess/MPC_FSEffect.MPC_FSEffect" "ToggleHighContrast")))
  (`GameUserSettings.SetVSyncEnabled` _returnvalue true))

(fn `UserConstructionScript`)