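; Base enemy Blueprint that provides Idle, Attack and FleePlayer actions, each signaling completion through its own end dispatcher.
; Idle alternates mesh materials on successive calls and Attack plays a punch animation, both finishing after short delays.
; FleePlayer checks the player against SafeDistance and, if too close, switches material and uses AIMoveTo to move directly away.
; Move success or failure both end the flee, restoring the material only at safe range.
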(event `Idle`
  (bind _mesh (`self.Mesh`))
  (`/Engine/EditorBlueprintResources/StandardMacros.FlipFlop`
    (:`A`
      (`PrimitiveComponent.SetMaterial` _mesh 0 "/Engine/VREditor/BasicMeshes/MI_Pyramid_01.MI_Pyramid_01")
      (`KismetSystemLibrary.Delay` 0.15)
      (`self.OnIdleEnd`))
    (:`B`
      (`PrimitiveComponent.SetMaterial` _mesh 0 "/Engine/Tutorial/SubEditors/TutorialAssets/Character/TutorialTPP_Mat.TutorialTPP_Mat")
      (`KismetSystemLibrary.Delay` 0.15)
      (`self.OnIdleEnd`))))

(event `Attack`
  (`SkeletalMeshComponent.PlayAnimation` (`self.Mesh`) "/Game/GameplayModules/Entities/Enemies/Punching_Anim_mixamo_com.Punching_Anim_mixamo_com" false)
  (`KismetSystemLibrary.Delay` 0.2)
  (`self.OnAttackEnd`))

(event `self.ReceiveBeginPlay`)

(event `FleePlayer`
  (bind _returnvalue (`self.K2_GetActorLocation` (`GameplayStatics.GetPlayerCharacter` 0)))
  (bind _returnvalue_2 (`self.K2_GetActorLocation` self))
  (if (>= (`self.SafeDistance`) (`KismetMathLibrary.Vector_Distance` _returnvalue_2 _returnvalue))
    (`PrimitiveComponent.SetMaterial` (`self.Mesh`) 0 "/Engine/EngineDebugMaterials/VertexColorViewMode_BlueOnly.VertexColorViewMode_BlueOnly")
    (`|AIMoveTo` self (+ (* (`KismetMathLibrary.GetDirectionUnitVector` _returnvalue _returnvalue_2) (`self.FleetingDistanceFactor`)) _returnvalue_2) null
      (:`OnSuccess`
        _)
      (:`OnFail`
        _))
    (if (>= (`KismetMathLibrary.Vector_Distance` (`self.K2_GetActorLocation` self) (`self.K2_GetActorLocation` (`GameplayStatics.GetPlayerCharacter` 0))) (`self.SafeDistance`))
      (`PrimitiveComponent.SetMaterial` (`self.Mesh`) 0 "/Engine/Tutorial/SubEditors/TutorialAssets/Character/TutorialTPP_Mat.TutorialTPP_Mat"))
    (`self.OnFleeEnd`)
    (else
      (`PrimitiveComponent.SetMaterial` (`self.Mesh`) 0 "/Engine/Tutorial/SubEditors/TutorialAssets/Character/TutorialTPP_Mat.TutorialTPP_Mat")
      (`self.OnFleeEnd`))))

(fn `UserConstructionScript`)