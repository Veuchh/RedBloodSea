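; BP_Dweller is an enemy with melee, projectile and flee behaviors that the player can possess or link to free it.
; It mirrors its AI state to the blackboard, choosing aggressive or afraid hair materials from the initial state.
; WeakpointsManager events drive hitstun and dissolving death; an Antagonist-tagged death alerts all Dwellers.
; PossessTarget events hide and restore it, or turn it Friendly and remove it once linked.
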(event `self.ReceiveBeginPlay`
  (bind _returnvalue (`AIBlueprintHelperLibrary.GetBlackboard` (`AIBlueprintHelperLibrary.GetAIController` self)))
  (`/Engine/EditorBlueprintResources/StandardMacros.IsValid` _returnvalue :!label _label
    (:`Is Valid`
      (`BlackboardComponent.SetValueAsObject` _returnvalue (`self.AttackTargetKeyName`) (`GameplayStatics.GetPlayerCharacter` 0))
      ;[1 1 1] Custom Stencil
      (`PrimitiveComponent.SetCustomDepthStencilValue` (`self.Mesh`) 254)
      (`PrimitiveComponent.SetCustomDepthStencilValue` (`self.DwellersHair`) 254)
      (for _array_element (`WeakpointsManager.MaterialInstances` (`self.WeakpointsManager`))
        (`MaterialInstanceDynamic.SetScalarParameterValue` _array_element "None" (`KismetMathLibrary.Conv_IntToDouble` (`KismetMathLibrary.RandomIntegerInRange` 1 3)))
        (switch `EAIStatesC` (`self.InitState`)
          (:`Aggressive`
            (set `self.AIState` "NewEnumerator0"))
          (:`Afraid`
            (set `self.AIState` "NewEnumerator1"))
          (:`Melee`
            (set `self.AIState` "NewEnumerator5"))
          (:`Distance`
            (set `self.AIState` "NewEnumerator6"))
          (:`Friendly`
            (set `self.AIState` "NewEnumerator2"))
          (:`Hitstun`
            (set `self.AIState` "NewEnumerator7"))
          (:`Dead`
            (set `self.AIState` "NewEnumerator3"))
          (:`DebugIdle`
            (set `self.AIState` "NewEnumerator4")))
        (`self.Set_AIStateToBlackboard` (`self.AIState`)))
      ;[1 1 1] Set Different parameters based on state for hair
      (switch `/Game/GameplayModules/Entities/Enemies/AI/Enums/E_AIStates` (`self.AIState`)
        (:`NewEnumerator0`
          (bind _returnvalue_2 (`KismetMaterialLibrary.CreateDynamicMaterialInstance` "/Game/Art/VFX/Mats/Dwellers/MI_HairAgressiv.MI_HairAgressiv" :!label _label_2))
          (set `self.DwellerHairMat` _returnvalue_2)
          (for _array_element_2 (`WeakpointsManager.MaterialInstances` (`self.WeakpointsManager`))
            (`MaterialInstanceDynamic.SetScalarParameterValue` _array_element_2 "AfraidOrAgressiv" 0.0)
            (`PrimitiveComponent.SetMaterial` (`self.DwellersHair`) 0 (`self.DwellerHairMat`) :!label _label_3)
            (bind _returnvalue_3 (`KismetMaterialLibrary.CreateDynamicMaterialInstance` "/Game/Art/VFX/Mats/Dwellers/AuraHair_Inst.AuraHair_Inst"))
            (`PrimitiveComponent.SetMaterial` (`self.StaticMesh`) 0 _returnvalue_3)
            (`BlackboardComponent.SetValueAsBool` (`AIBlueprintHelperLibrary.GetBlackboard` (`AIBlueprintHelperLibrary.GetAIController` self)) (`self.ShouldPatrolKeyName`) (`self.ShouldPatrol`))))
        (:`NewEnumerator1`
          (bind _returnvalue_4 (`KismetMaterialLibrary.CreateDynamicMaterialInstance` "/Game/Art/VFX/Mats/Dwellers/MI_HairAfraid.MI_HairAfraid" :!label _label_4))
          (set `self.DwellerHairMat` _returnvalue_4)
          (for _array_element_3 (`WeakpointsManager.MaterialInstances` (`self.WeakpointsManager`))
            (`MaterialInstanceDynamic.SetScalarParameterValue` _array_element_3 "AfraidOrAgressiv" 1.0)
            (goto _label_3)))
        (:`NewEnumerator2`
          (goto _label_4))
        (:`NewEnumerator5`
          (goto _label_2))
        (:`NewEnumerator6`
          (goto _label_4))))
    (:`Is Not Valid`
      (`KismetSystemLibrary.DelayUntilNextTick`)
      (goto _label))))

(event `self.WeakpointsManager.OnWeakpointReveal`
  (bind _mesh (`self.Mesh`))
  (bind _am_stun (`self.AM_Stun`))
  (`MaterialInstanceDynamic.SetScalarParameterValue` (`self.DwellerHairMat`) "MaskAnim" 0.0)
  (`ActorComponent.Activate` (`self.FX_DwellerSlashed`) false)
  (switch `int` (`KismetMathLibrary.RandomInteger` 3)
    (:`0`
      (`|PlayMontage` _mesh "/Game/GameplayModules/Entities/Enemies/Anim/AnimsHugo/AM_Hit1Hugo.AM_Hit1Hugo"
        (:`then`
          (if (`|EnumInequality` (cast `/Game/GameplayModules/Entities/Enemies/AI/Enums/E_AIStates` (`BlackboardComponent.GetValueAsEnum` (`AIBlueprintHelperLibrary.GetBlackboard` (`AIBlueprintHelperLibrary.GetAIController` self)) (`self.AIStateKeyName`))) "NewEnumerator7") :!label _label_5
            (`self.Get_AIStateFromBlackboard`)
            (`self.Set_AIStateToBlackboard` "NewEnumerator7")
            (bind (_direction _hitscaleanim) (`Timeline|HairHit` :!via `PlayFromStart` :!label _label_6)
              (:`Update`
                (`MaterialInstanceDynamic.SetScalarParameterValue` (`self.DwellerHairMat`) "ScaleAnimation" (* _hitscaleanim 4.0))))
            (else
              (goto _label_6 :!via `PlayFromStart`))))
        (:`OnBlendOut`
          (`|PlayMontage` (`self.Mesh`) _am_stun :!label _label_7
            (:`then`
              (`TimelineComponent.SetPlayRate` (`self.HairStunAnimation`) (`self.HitstunDuration`))
              (bind (_direction_2 _hairanimation) (`Timeline|HairStunAnimation` :!via `PlayFromStart`)
                (:`Update`
                  (`MaterialInstanceDynamic.SetScalarParameterValue` (`self.DwellerHairMat`) "MaskAnim" _hairanimation))
                (:`Finished`
                  (`KismetSystemLibrary.Delay` (`self.HitstunDuration`))
                  (`self.StopAnimMontage` _am_stun)
                  (`self.Set_AIStateToBlackboard` (`self.AIState`))
                  (cast `/Game/GameplayModules/Entities/Enemies/AI/AIC_EnemyBase` (`AIBlueprintHelperLibrary.GetAIController` self)))))))))
    (:`1`
      (`|PlayMontage` _mesh "/Game/GameplayModules/Entities/Enemies/Anim/AnimsHugo/AM_Hit2Hugo.AM_Hit2Hugo"
        (:`then`
          (goto _label_5))
        (:`OnBlendOut`
          (goto _label_7))))
    (:`2`
      (`|PlayMontage` _mesh "/Game/GameplayModules/Entities/Enemies/Anim/AnimsHugo/AM_Hit3Hugo.AM_Hit3Hugo"
        (:`then`
          (goto _label_5))
        (:`OnBlendOut`
          (goto _label_7))))))

(event `self.WeakpointsManager.OnWeakpointHit`
  (params (Weakpoint :type "Actor Object Reference"))
  (bind _returnvalue (`self.K2_GetActorLocation` Weakpoint))
  (`NiagaraFunctionLibrary.SpawnSystemAtLocation` "/Game/Art/VFX/ParticlesSystems/FX_WeakPointsExplo.FX_WeakPointsExplo" _returnvalue (`KismetMathLibrary.Quat_Rotator` (* (`KismetMathLibrary.Conv_RotatorToQuaternion` (`KismetMathLibrary.FindLookAtRotation` _returnvalue (`self.K2_GetActorLocation` (`GameplayStatics.GetPlayerCameraManager` 0)))) (`KismetMathLibrary.Conv_RotatorToQuaternion` (`KismetMathLibrary.MakeRotator` (`KismetMathLibrary.RandomFloatInRange` -5.0 5.0) (+ (`KismetMathLibrary.RandomFloatInRange` -5.0 5.0) -90.0))))) (`KismetMathLibrary.Conv_DoubleToVector` 0.3)))

(event `LaunchProjectile`
  (bind _returnvalue (+ (`self.K2_GetActorLocation`) (0.0 0.0 100.0)))
  (bind _returnvalue_2 (`KismetMathLibrary.RandomFloatInRange` (* (`self.DwellerAimOffset`) -1.0) (`self.DwellerAimOffset`)))
  (bind _outhit (`KismetSystemLibrary.LineTraceSingleForObjects` (`self.K2_GetActorLocation`) (`self.K2_GetActorLocation` (`GameplayStatics.GetPlayerCharacter` 0)) (`|MakeArray` "ObjectTypeQuery3" "ObjectTypeQuery1" :!type "EObjectTypeQuery Enum")))
  (if (== (`.HitActor` (`GameplayStatics.BreakHitResult` _outhit)) (`GameplayStatics.GetPlayerCharacter` 0))
    (`AkGameplayStatics.PostEvent` "/Game/WwiseAudio/Events/Default_Work_Unit/Ai_Behavior/Play_EnemyProjectileCast.Play_EnemyProjectileCast" self)
    (`|PlayMontage` (`self.Mesh`) "/Game/GameplayModules/Entities/Enemies/Anim/AM_Throw.AM_Throw"
      (:`OnCompleted`
        (`self.OnProjectileEnd` :!label _label_8))
      (:`OnInterrupted`
        (goto _label_8))
      (:`OnNotifyBegin`
        (`|SpawnActorFromClass` "/Game/GameplayModules/Entities/Enemies/Projectile/BP_Projectile.BP_Projectile_C" (`KismetMathLibrary.MakeTransform` _returnvalue (`KismetMathLibrary.FindLookAtRotation` _returnvalue (+ (`self.K2_GetActorLocation` (`GameplayStatics.GetPlayerCharacter` 0)) (`KismetMathLibrary.MakeVector` _returnvalue_2 _returnvalue_2)))) "AlwaysSpawn" "MultiplyWithRoot" null null)))
    (else
      (`self.OnProjectileEnd`))))

(event `MeleeAttack`
  (bind _returnvalue (`self.K2_GetActorLocation`))
  (bind _meleeduration (`self.MeleeDuration`))
  (`|PlayMontage` (`self.Mesh`) "/Game/GameplayModules/Entities/Enemies/Anim/AnimsHugo/AM_AngryMelee.AM_AngryMelee"
    (:`then`
      (`KismetSystemLibrary.Delay` _meleeduration)
      (`self.OnAttackEnd`))
    (:`OnNotifyBegin`
      (bind (_outhit _returnvalue_2) (`KismetSystemLibrary.SphereTraceSingleForObjects` :`Start` _returnvalue :`End` (+ _returnvalue (* (`self.GetActorForwardVector`) (`self.MeleeColliderLength`))) :`Radius` (`self.MeleeColliderRadius`) :`ObjectTypes` (`|MakeArray` "ObjectTypeQuery3" :!type "EObjectTypeQuery Enum") :`DrawDebugType` "ForDuration" :`DrawTime` _meleeduration))
      (if _returnvalue_2
        (bind _asred_blood_sea_character (cast `RedBloodSeaCharacter` (`.HitActor` (`GameplayStatics.BreakHitResult` _outhit))))
        (`PlayerCombat.DamagePlayer` (`self.GetComponentByClass` _asred_blood_sea_character "/Script/RedBloodSea.PlayerCombat") (`self.MeleeDamage`) self)))))

(event `FleePlayer`
  (bind _returnvalue (`self.K2_GetActorLocation` self))
  (`|AIMoveTo` self (+ (* (`KismetMathLibrary.GetDirectionUnitVector` (`self.K2_GetActorLocation` (`GameplayStatics.GetPlayerCharacter` 0)) _returnvalue) (`self.FleetingDistanceFactor`)) _returnvalue) null
    (:`OnSuccess`
      _)
    (:`OnFail`
      _))
  (`self.OnFleeEnd`))

(event `self.PossessTarget.OnPossessed`
  (`self.SetActorEnableCollision` false)
  (`self.SetActorHiddenInGame` true)
  (`self.SetActorTickEnabled` false))

(event `self.PossessTarget.OnUnpossessed`
  (params (RepositionEnemyAtPosition :type "Vector Structure"))
  (`self.K2_SetActorLocation` RepositionEnemyAtPosition)
  (`self.SetActorEnableCollision` true)
  (`self.SetActorHiddenInGame` false)
  (`self.SetActorTickEnabled` true)
  (`self.Set_AIStateToBlackboard` (`self.AIState`)))

(event `self.WeakpointsManager.OnDeath`
  (params (Dweller :type "Actor Object Reference"))
  (`self.Set_AIStateToBlackboard` "NewEnumerator3")
  (`|PlayMontage` (`self.Mesh`) "/Game/GameplayModules/Entities/Enemies/Anim/AnimsHugo/AM_DeathHugo.AM_DeathHugo"
    (:`then`
      (if (`self.ActorHasTag` "Antagonist")
        (bind _outactors (`GameplayStatics.GetAllActorsOfClass` "BP_Dweller_C"))
        (for _array_element _outactors
          (`BlackboardComponent.SetValueAsBool` (`AIBlueprintHelperLibrary.GetBlackboard` (`AIBlueprintHelperLibrary.GetAIController` _array_element)) (`self.SawAntagonistDeathKeyName`) true)
          ;[1 1 1] Activate Death FX
          (`ActorComponent.Activate` (`self.FX_DwellerDeath`) false :!label _label_9)
          (`AkGameplayStatics.PostEvent` "/Game/WwiseAudio/Events/Default_Work_Unit/Ai_Behavior/Play_EnemyDeath.Play_EnemyDeath" Dweller)
          ;[1 1 1] DeathEvent
          (bind (_direction _dissolve _hairdissolve) (`Timeline|Dissolve`)
            (:`Update`
              (`MaterialInstanceDynamic.SetScalarParameterValue` (`self.DwellerHairMat`) "MaskDissolve" _hairdissolve)
              (for _array_element_2 (`WeakpointsManager.MaterialInstances` (`self.WeakpointsManager`))
                (`MaterialInstanceDynamic.SetScalarParameterValue` _array_element_2 "DissolveAmount" _dissolve)))
            (:`Finished`
              (`KismetSystemLibrary.Delay` 0.4)
              (`self.K2_DestroyActor` Dweller))))
        (else
          (goto _label_9))))
    (:`OnCompleted`
      (`|PlayMontage` (`self.Mesh`) "/Game/GameplayModules/Entities/Enemies/Anim/AnimsHugo/AM_DeathPose.AM_DeathPose" 0.0 :!label _label_10))
    (:`OnBlendOut`
      (goto _label_10))))

(event `self.PossessTarget.OnLinked`
  (params (Actor :type "Actor Object Reference"))
  (`AkGameplayStatics.PostEvent` "/Game/WwiseAudio/Events/Default_Work_Unit/Ai_Behavior/Play_EnemyFreed.Play_EnemyFreed" Actor)
  (`UDataSubsystem.AddLinked` (subsystem `UDataSubsystem`) 1)
  (`self.Set_AIStateToBlackboard` "NewEnumerator2")
  (`ActorComponent.Activate` (`self.FX_LinkComplete`) false)
  (`KismetSystemLibrary.Delay` 1.0)
  (`SceneComponent.SetVisibility` (`self.Mesh`) false true)
  (`KismetSystemLibrary.Delay` 2.0)
  (`self.K2_DestroyActor`))

(event `self.PossessTarget.OnPrepareForPossess`
  (`self.Get_AIStateFromBlackboard`)
  (`self.Set_AIStateToBlackboard` "NewEnumerator2"))

(fn `Get_AIStateFromBlackboard`
  (bind _asaic_enemy_base (cast `/Game/GameplayModules/Entities/Enemies/AI/AIC_EnemyBase` (`AIBlueprintHelperLibrary.GetAIController` self)))
  (bind _blackboardcomponent (`AIController.UseBlackboard` _asaic_enemy_base "/Game/GameplayModules/Entities/Enemies/AI/BB_EnemyBase.BB_EnemyBase"))
  (set `self.AIState` (cast `/Game/GameplayModules/Entities/Enemies/AI/Enums/E_AIStates` (`BlackboardComponent.GetValueAsEnum` _blackboardcomponent (`self.AIStateKeyName`)))))

(fn `Set_AIStateToBlackboard`
  (params (StateToSet :type "/Game/GameplayModules/Entities/Enemies/AI/Enums/E_AIStates Enum" :default "NewEnumerator0"))
  (locals (StateKeyName :type Name :default "State"))
  (bind _asaic_enemy_base (cast `/Game/GameplayModules/Entities/Enemies/AI/AIC_EnemyBase` (`AIBlueprintHelperLibrary.GetAIController` self)))
  (`BlackboardComponent.SetValueAsEnum` (`AIBlueprintHelperLibrary.GetBlackboard` _asaic_enemy_base) (`self.AIStateKeyName`) StateToSet))

(fn `UserConstructionScript`)