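; BP_SpawnerManager is the Blueprint layer of the wave spawner, reacting to wave events with HUD, audio switch and player updates.
; On BeginPlay it caches BP_HUD and binds wave start, success, fail and objective-update events, which set or clear the HUD objective and toggle combat/between-wave switches.
; Start and success also set the wave-index switch; failure destroys the player character.
; EndPlay stores objective completion and timing in the data subsystem.
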(event `self.ReceiveBeginPlay`
  (bind _asbp_hud (cast `/Game/GameplayModules/UI/BP_HUD` (`PlayerController.GetHUD` (`GameplayStatics.GetPlayerController` 0))))
  (set `self.PlayerHUD` _asbp_hud)
  (add `self.OnWaveFail` (delegate `OnWaveFail_Event`))
  (add `self.OnWaveStart` (delegate `OnWaveStart_Event`))
  (add `self.OnUpdateObjective` (delegate `OnUpdateObjective_Event`))
  (add `self.OnWaveSuccess` (delegate `OnWaveSuccess_Event`)))

(event `OnUpdateObjective_Event` :!signature `self.OnUpdateObjective`
  (params (Wave :type "Wave Structure (by ref)"))
  (`/Game/GameplayModules/UI/BP_HUD.SetObjective` (`self.PlayerHUD`) Wave))

(event `OnWaveSuccess_Event`
  (`AkGameplayStatics.SetSwitch` "/Game/WwiseAudio/Switches/Default_Work_Unit/switch_combat_phase/switch_combat_status-between_wave.switch_combat_status-between_wave")
  (`/Game/GameplayModules/UI/BP_HUD.RemoveObjective` (`self.PlayerHUD`))
  (`AkGameplayStatics.SetSwitch` null null "switch_combat_wave_index" :!label _label))

(event `OnWaveFail_Event`
  (`AkGameplayStatics.SetSwitch` "/Game/WwiseAudio/Switches/Default_Work_Unit/switch_combat_phase/switch_combat_status-between_wave.switch_combat_status-between_wave")
  (`self.K2_DestroyActor` (`GameplayStatics.GetPlayerCharacter` 0))
  (`/Game/GameplayModules/UI/BP_HUD.RemoveObjective` (`self.PlayerHUD`)))

(event `OnWaveStart_Event`
  (`AkGameplayStatics.SetSwitch` "/Game/WwiseAudio/Switches/Default_Work_Unit/switch_combat_phase/switch_combat_status-combat.switch_combat_status-combat")
  (goto _label))

(event `self.ReceiveEndPlay`
  (params (EndPlayReason :type "EEndPlayReason Enum" :default "Destroyed"))
  (bind _returnvalue (subsystem `UDataSubsystem`))
  (`UDataSubsystem.StoreObjectiveCompletion` _returnvalue (`self.Waves`))
  (set `UDataSubsystem.StartTime` (`self.StartTime`) _returnvalue)
  (set `UDataSubsystem.EndTime` (`self.EndTime`) _returnvalue))

(fn `NewFunction`)

(fn `UserConstructionScript`)