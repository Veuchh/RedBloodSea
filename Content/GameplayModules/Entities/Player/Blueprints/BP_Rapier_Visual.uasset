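; Visual actor for the player's rapier, switching the blade and its ribbon between an HC state and a neutral state.
; BeginPlay creates dynamic materials for both meshes.
; MorphtoHC and MorphtoNeutral set IsHC and play timelines driving the ribbon's morph target, its isHC parameter and the blade's core glow.
; Linking plays a timeline that animates the morph target while holding link glow at zero, without checking IsHC.
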(event `self.ReceiveBeginPlay`
  (bind _sm_rapier (`self.SM_Rapier`))
  (bind _returnvalue (`PrimitiveComponent.CreateDynamicMaterialInstance` (`self.RapierRibbonBlendSHape`) 0 "/Game/Art/Characters/Mat/MI_RapierRibbon.MI_RapierRibbon" "None"))
  (bind _output_get (set `self.RibbonMat` _returnvalue))
  (`PrimitiveComponent.SetMaterial` (`self.RapierRibbonBlendSHape`) 0 _output_get)
  (bind _returnvalue_2 (`PrimitiveComponent.CreateDynamicMaterialInstance` _sm_rapier 0 "/Game/Art/Characters/Mat/MI_Rapier.MI_Rapier" "None"))
  (bind _output_get_2 (set `self.RapierMat` _returnvalue_2))
  (`PrimitiveComponent.SetMaterial` _sm_rapier 0 _output_get_2))

(event `MorphtoHC`
  (set `self.isHC` true)
  (bind (_direction _morphtarget _lightmap _bladeglow) (`Timeline|HCMorph` :!via `PlayFromStart`)
    (:`Update`
      (`SkeletalMeshComponent.SetMorphTarget` (`self.RapierRibbonBlendSHape`) "attribblur1" _morphtarget true)
      (`MaterialInstanceDynamic.SetScalarParameterValue` (`self.RibbonMat`) "isHC" _lightmap)
      (`MaterialInstanceDynamic.SetScalarParameterValue` (`self.RapierMat`) "CoreGlow_Amount" _bladeglow))))

(event `MorphtoNeutral`
  (set `self.isHC` false)
  (bind (_direction _morph _bladeglow _ribbonmode) (`Timeline|NeutralMorph` :!via `PlayFromStart`)
    (:`Update`
      (`SkeletalMeshComponent.SetMorphTarget` (`self.RapierRibbonBlendSHape`) "attribblur1" _morph true)
      (`MaterialInstanceDynamic.SetScalarParameterValue` (`self.RibbonMat`) "isHC" _bladeglow)
      (`MaterialInstanceDynamic.SetScalarParameterValue` (`self.RapierMat`) "CoreGlow_Amount" _ribbonmode))))

(event `Linking`
  (bind (_direction _morphifhc) (`Timeline|LinkingAnim` :!via `PlayFromStart`)
    (:`Update`
      (if true
        (`SkeletalMeshComponent.SetMorphTarget` (`self.RapierRibbonBlendSHape`) "attribblur1" _morphifhc true)
        (`MaterialInstanceDynamic.SetScalarParameterValue` (`self.RapierMat`) "LinkGlow_Amount" 0.0)))))

(fn `UserConstructionScript`)