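; BP_Dweller is an enemy in the weak point test module that exposes its weak points when the player character overlaps it.
; On BeginPlay its mesh loops a forward run animation.
; The first overlap with a RedBloodSeaCharacter calls RevealWeakpoints on the WeakpointsManager, guarded by a Revealed flag.
; The reveal and hit event handlers are empty, and the logic to face the player is disconnected.
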(event `self.ReceiveBeginPlay`
  (`SkeletalMeshComponent.PlayAnimation` (`self.Mesh`) "/Game/GameplayModules/Entities/Enemies/Characters/Mannequins/Animations/Manny/MM_Run_Fwd.MM_Run_Fwd" true))

(event `self.ReceiveTick`
  (params (DeltaSeconds :type "Float (single-precision)")))

(event `self.ReceiveActorBeginOverlap`
  (params (OtherActor :type "Actor Object Reference"))
  (if (not (`self.Revealed`))
    (cast `RedBloodSeaCharacter` OtherActor)
    (`WeakpointsManager.RevealWeakpoints` (`self.WeakpointsManager`))
    (set `self.Revealed` true)))

(event `self.WeakpointsManager.OnWeakpointReveal`
  (params (Character :type "Actor Object Reference")))

(event `self.WeakpointsManager.OnWeakpointHit`
  (params (Character :type "Actor Object Reference") (Weakpoint :type "Actor Object Reference")))

(fn `UserConstructionScript`)