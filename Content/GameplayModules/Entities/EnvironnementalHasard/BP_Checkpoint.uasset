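; Checkpoint actor that gives audio and visual feedback, with no respawn or save logic in its graph.
; A Wwise loop starts on BeginPlay, and Tick smoothly turns FXCheckPoint on yaw only to face player 0's character.
; The first overlap of Collider by the player pawn posts the crossed sound through a DoOnce, which is never reset.
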(event `self.ReceiveBeginPlay`
  (`AkGameplayStatics.PostEvent` "/Game/WwiseAudio/Events/Default_Work_Unit/Play_CheckpointLoop.Play_CheckpointLoop" self))

(event `self.ReceiveTick`
  (params (DeltaSeconds :type "Float (single-precision)"))
  (bind _returnvalue (`GameplayStatics.GetPlayerCharacter` 0))
  (bind _fx_checkpoint (`self.FX_CheckPoint`))
  (bind _returnvalue_2 (`SceneComponent.K2_GetComponentRotation` _fx_checkpoint))
  (bind (_returnvalue_roll _returnvalue_pitch _returnvalue_yaw) (`KismetMathLibrary.BreakRotator` (`KismetMathLibrary.RInterpTo` _returnvalue_2 (`KismetMathLibrary.FindLookAtRotation` (`SceneComponent.K2_GetComponentLocation` _fx_checkpoint) (`self.K2_GetActorLocation` _returnvalue)) (`GameplayStatics.GetWorldDeltaSeconds`) 5.0)))
  (`/Engine/EditorBlueprintResources/StandardMacros.IsValid` _returnvalue
    (:`Is Valid`
      (`SceneComponent.K2_SetWorldRotation` _fx_checkpoint (`KismetMathLibrary.MakeRotator` (.roll _returnvalue_2) (.pitch _returnvalue_2) _returnvalue_yaw) false false))))

(event `self.Collider.OnComponentBeginOverlap`
  (params (OverlappedComponent :type "PrimitiveComponent Object Reference") (OtherActor :type "Actor Object Reference") (OtherComp :type "PrimitiveComponent Object Reference") (OtherBodyIndex :type Integer) (bFromSweep :type Boolean) (SweepResult :type "HitResult Structure (by ref)"))
  (if (== OtherActor (`GameplayStatics.GetPlayerPawn` 0))
    (`/Engine/EditorBlueprintResources/StandardMacros.DoOnce` false
      (:`Completed`
        (`AkGameplayStatics.PostEvent` "/Game/WwiseAudio/Events/Default_Work_Unit/Play_CheckpointCrossed.Play_CheckpointCrossed" self)))))

(fn `UserConstructionScript`)