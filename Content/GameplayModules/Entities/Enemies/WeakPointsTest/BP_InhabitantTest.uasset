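; Test enemy that plays a looping run animation, keeps rotating to face the player and carries randomly placed weak points.
; On BeginPlay it gathers mesh sockets with "wp_" in their names, then spawns and attaches a configurable number of BP_WeakPoint actors to them.
; Each chosen socket moves from the available pool to a used list, so no socket is picked twice.
; Tick applies the look-at rotation with a fixed 90-degree offset.
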(event `self.ReceiveBeginPlay`
  (`SkeletalMeshComponent.PlayAnimation` (`self.Mesh`) "/Game/GameplayModules/Entities/Enemies/Characters/Mannequins/Animations/Manny/MM_Run_Fwd.MM_Run_Fwd" true)
  (for _array_element (`SceneComponent.GetAllSocketNames` (`self.Mesh`))
    (if (`KismetStringLibrary.Contains` (`KismetStringLibrary.Conv_NameToString` _array_element) "wp_")
      (`KismetArrayLibrary.Array_Add` (`self.Sockets_WeakPoints`) _array_element)))
  (for _ (range (`self.Nb_WeakPoints`))
    (`self.CreateNewWeakPoint`)))

(event `self.ReceiveTick`
  (params (DeltaSeconds :type "Float (single-precision)"))
  (`self.K2_SetActorRotation` (`KismetMathLibrary.ComposeRotators` (`KismetMathLibrary.FindLookAtRotation` (`self.K2_GetActorLocation`) (`self.K2_GetActorLocation` (`GameplayStatics.GetPlayerCharacter` 0))) (struct :`Yaw` -90.0))))

(fn `CreateNewWeakPoint`
  (locals (Weakpoint :type Name))
  (bind _weakpoint (`local.Weakpoint`))
  (bind _sockets_weakpoints (`self.Sockets_WeakPoints`))
  (if (`KismetArrayLibrary.Array_IsNotEmpty` _sockets_weakpoints)
    (bind _output_get (set `local.Weakpoint` (`KismetArrayLibrary.Array_Random` _sockets_weakpoints)))
    (bind _returnvalue (`|SpawnActorFromClass` "/Game/GameplayModules/Entities/Enemies/WeakPointsTest/BP_WeakPoint.BP_WeakPoint_C" (`SceneComponent.GetSocketTransform` (`self.Mesh`) _output_get "RTS_ParentBoneSpace") "Undefined" "MultiplyWithRoot" null null))
    (`self.K2_AttachToComponent` _returnvalue (`self.Mesh`) (`local.Weakpoint`) "SnapToTarget" "SnapToTarget" "KeepRelative" false)
    (`KismetArrayLibrary.Array_RemoveItem` (`self.Sockets_WeakPoints`) _weakpoint)
    (`KismetArrayLibrary.Array_Add` (`self.UsedSockets_Weakpoints`) _weakpoint)))

(fn `UserConstructionScript`)